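; BP_StepManager tracks the current step of a simulation and checks that objects are clicked in the required order.
; CheckInteraction takes the clicked object's ID and compares it to the TargetID in the StepDataTable row named from the current step index.
; A match advances CurrentStep and returns true; a mismatch returns false, with a success or retry message printed either way.
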(fn `CheckInteraction`
  (params (ClickedID :type Name))
  (returns (IsCompleted :type Boolean))
  (locals (NewLocalVar :type Text))
  ; 단계확인 노드 -> 시뮬레이션 순서가 맞는지 확인하고 클릭한거랑 순서가 다를 때 판단
  ;; 물체 클릭시 호출
  (bind _returnvalue (`|GetDataTableRow` (`self.StepDataTable`) (`KismetStringLibrary.Conv_StringToName` (`KismetTextLibrary.Conv_TextToString` (`|FormatText` "Step{Index}" (`self.CurrentStep`)))))
    (:`then`
      (if (== ClickedID (`.TargetID_5_9CF49BCD4EC6907FE0F5EBBCEE43A712` (break `/Game/Blueprints/Struct/ST_Step` _returnvalue)))
        (`KismetSystemLibrary.PrintString` "성공")
        (`/Engine/EditorBlueprintResources/StandardMacros.IncrementInt` (`self.CurrentStep`)
          (:`  `
            (return true)))
        (else
          (`KismetSystemLibrary.PrintString` "다시 고르기")
          (return false))))))

(fn `UserConstructionScript`)